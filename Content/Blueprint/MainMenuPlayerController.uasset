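; Main menu player controller that hosts a party session for the player and lists discoverable sessions as debug text.
; On BeginPlay it creates a two-slot Advanced Sessions session tagged Type=Party, then reopens MainMenu as a listen server.
; Every Tick it starts an unfiltered session search across all server types and prints each found server name for one frame's duration.
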(event Custom|Host%20Party
  (|AdvancedSession (Utilities|Array|MakeArray (Class|AdvancedSessionsLibrary|MakeLiteralSessionPropertyString "Type" "Party")) (Game|GetPlayerController 0) 2 0 false true false true true false true false true
    (:OnSuccess
      (Game|OpenLevel(byName) "MainMenu" true "listen")
      (Development|PrintString "Created party!" true true "(R=0.191297,G=1.000000,B=0.000000,A=1.000000)" 5.0))
    (:OnFailure
      (Development|PrintString "Lobby Creation Failed" true true "(R=1.000000,G=0.030466,B=0.000000,A=1.000000)" 5.0))))

(event EventBeginPlay
  (CallFunction|HostParty))

(event EventTick
  (params (DeltaSeconds :type Float%20%28single-precision%29))
  (bind _results (|FindSessionsAdvanced self 10 false "AllServers" 0 false false false)
    (:OnSuccess
      (for _array_element _results
        (Development|PrintString (Utilities|String|Append "Found server: " (Class|FindSessionsCallbackProxy|GetServerName _array_element)) true true "(R=0.000000,G=0.660000,B=1.000000,A=1.000000)" DeltaSeconds))
      (Development|PrintString "Finished showing servers." true true "(R=0.000000,G=0.660000,B=1.000000,A=1.000000)" DeltaSeconds))
    (:OnFailure
      (Development|PrintString "Failed to find servers"))))

(fn ConstructionScript)